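; GI_IO is a Game Instance that owns the player's user settings save object and handles its persistence.
; On Init it loads the UserSettings slot into UserSave, or creates a fresh Save_UserSettings object in memory when no save exists.
; A separate SaveUserSettings event writes UserSave back to that slot.
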(event `self.ReceiveInit`
  (`self.Load User Settings`))

(event `Load User Settings`
  ;[1 1 1] User settings
  (bind _returnvalue (`GameplayStatics.DoesSaveGameExist` "UserSettings"))
  (if _returnvalue
    (bind _returnvalue_2 (`GameplayStatics.LoadGameFromSlot` "UserSettings"))
    (bind _assave_user_settings (cast `/Game/Blueprints/ModesAndInstance/Save_UserSettings` _returnvalue_2))
    (set `self.UserSave` _assave_user_settings)
    (else
      (bind _returnvalue_3 (`GameplayStatics.CreateSaveGameObject` "/Game/Blueprints/ModesAndInstance/Save_UserSettings.Save_UserSettings_C"))
      (set `self.UserSave` _returnvalue_3))))

(event `Save User Settings`
  ;[1 1 1] User settings
  (`GameplayStatics.SaveGameToSlot` (`self.UserSave`) "UserSettings"))