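; GM_Menu is the main menu game mode, which sets up the menu UI and camera view when a player logs in.
; PostLogin adds a UMG_MainMenu widget to the viewport, then after a short delay stores it on the controlled Char_IO pawn.
; If that cast succeeds, it loops over CameraActors, skips those owned by player 0's camera manager, and sets each remaining one as view target, so the last wins.
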(event `self.K2_PostLogin`
  (params (NewPlayer :type "PlayerController Object Reference"))
  (bind _returnvalue (`|CreateWidget` "/Game/Widgets/UMG_MainMenu.UMG_MainMenu_C" NewPlayer))
  (`UserWidget.AddToViewport` _returnvalue 0)
  (`KismetSystemLibrary.Delay` 0.2)
  (bind _aschar_io (cast `/Game/Blueprints/Player/Char_IO` (`Controller.K2_GetPawn` NewPlayer)))
  (set `/Game/Blueprints/Player/Char_IO.MainMenu` _returnvalue _aschar_io)
  (bind _outactors (`GameplayStatics.GetAllActorsOfClass` "/Script/Engine.CameraActor"))
  (for _array_element _outactors
    (if (not (== (`self.GetOwner` _array_element) (`GameplayStatics.GetPlayerCameraManager` 0)))
      (`PlayerController.SetViewTargetWithBlend` NewPlayer _array_element 0.0 "VTBlend_Linear" 0.0 false))))

(fn `UserConstructionScript`)