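; Interactable terminal actor from which the player recovers a data file.
; Focus shows a powered or power-required message based on its Powered flag, and losing focus resets the player's inventory menu.
; Activating always shows a "Data Found!" message without checking Powered.
; The first successful activation adds a data file through GM_Game and sets Used, so it counts only once.
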(event `/Game/Blueprints/Crafting/Interface_Interact.Activate Interact`
  (params (PlayerPawn :type "/Game/Blueprints/Player/Char_IO Object Reference"))
  (`/Game/Blueprints/Player/Char_IO.Menu Message` PlayerPawn "Data Found!" "Data has been transmitted to pod.")
  (if (not (`self.Used`))
    (bind _asgm_game (cast `/Game/Blueprints/ModesAndInstance/GM_Game` (`GameplayStatics.GetGameMode`)))
    (`/Game/Blueprints/ModesAndInstance/GM_Game.Add Data File` _asgm_game)
    (set `self.Used` true)))

(event `/Game/Blueprints/Crafting/Interface_Interact.EndFocus Interact`
  (params (PlayerPawn :type "/Game/Blueprints/Player/Char_IO Object Reference"))
  (`/Game/Blueprints/Player/Char_IO.Reset Inventory Menu` PlayerPawn))

(event `/Game/Blueprints/Crafting/Interface_Interact.StartFocus Interact`
  (params (PlayerPawn :type "/Game/Blueprints/Player/Char_IO Object Reference"))
  (if (`self.Powered`)
    (`/Game/Blueprints/Player/Char_IO.Menu Message` PlayerPawn "Terminal Powered" "Terminal is powered. Interact to recover data.")
    (else
      (`/Game/Blueprints/Player/Char_IO.Menu Message` PlayerPawn "Power required" "There is a faint signal here, however power is required to retreive data."))))

(fn `UserConstructionScript`)