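; Drop pod pawn that delivers a player by falling to the ground and building their Char_IO character.
; Possession starts a manual fall on Tick, moving the pod downward until a short line trace hits a surface.
; Landing plays the opening animation, then shows a beam and rover mesh while a timeline drives the burnable material's Amount.
; When the timeline finishes, both hide and the authority spawns Char_IO and transfers possession.
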(event `self.ReceivePossessed`
  (params (NewController :type "Controller Object Reference"))
  (set `self.Gravity` true))

(event `self.ReceiveBeginPlay`
  (bind _rover_build (`self.Rover Build`))
  (`SceneComponent.SetVisibility` (`self.Beam`) false false)
  (`SceneComponent.SetVisibility` _rover_build false false)
  (bind _returnvalue (`PrimitiveComponent.CreateDynamicMaterialInstance` _rover_build 0 "/Game/Materials/Burnable/Burnable_Mat_Inst.Burnable_Mat_Inst" "None"))
  (bind _output_get (set `self.BuildMat` _returnvalue))
  (`MaterialInstanceDynamic.SetScalarParameterValue` _output_get "Amount" 1.0))

(event `self.ReceiveTick`
  (params (DeltaSeconds :type "Float (single-precision)"))
  (bind _returnvalue (`self.K2_GetActorLocation`))
  (if (`self.Gravity`)
    (`self.K2_AddActorWorldOffset` (0.0 0.0 -30.0))
    (bind (_outhit _returnvalue_2) (`KismetSystemLibrary.LineTraceSingle` :`Start` _returnvalue :`End` (+ _returnvalue (0.0 0.0 -30.0)) :`TraceChannel` "TraceTypeQuery1" :`DrawDebugType` "ForDuration"))
    (if _returnvalue_2
      (`/Engine/EditorBlueprintResources/StandardMacros.DoOnce` false
        (:`Completed`
          (set `self.Gravity` false)
          (`SkeletalMeshComponent.PlayAnimation` (`self.SkeletalMesh`) "/Game/Mesh/DropPod/DropPod_Anim_Armature_LandingandOpening.DropPod_Anim_Armature_LandingandOpening" false)
          (`KismetSystemLibrary.Delay` 2.0)
          (`SceneComponent.SetVisibility` (`self.Beam`) true false)
          (`SceneComponent.SetVisibility` (`self.Rover Build`) true false)
          (bind (_direction _newtrack_0) (`Timeline|Timeline_0` :!via `PlayFromStart`)
            (:`Update`
              (`MaterialInstanceDynamic.SetScalarParameterValue` (`self.BuildMat`) "Amount" _newtrack_0))
            (:`Finished`
              (`SceneComponent.SetVisibility` (`self.Rover Build`) false false)
              (`SceneComponent.SetVisibility` (`self.Beam`) false false)
              (`/Engine/EditorBlueprintResources/ActorMacros.Switch Has Authority`
                (:`Authority`
                  (bind _returnvalue_3 (`|SpawnActorFromClass` "/Game/Blueprints/Player/Char_IO.Char_IO_C" (`SceneComponent.K2_GetComponentToWorld` (`self.Rover Build`)) "AlwaysSpawn" "OverrideRootScale" null self))
                  (`Controller.Possess` (`self.GetController`) _returnvalue_3))))))))))

(fn `UserConstructionScript`)