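; Player rover character driven entirely by two buttons, which handle movement, menus, interaction and building.
; Holds drive or turn the rover with animated treads and ground alignment, while taps fill a buffer matched against combo strings to navigate and select.
; A timer loop traces for Interface_Interact targets or positions a craft preview in build mode.
; It also runs a timed tutorial and collects harvested resources up to a shared capacity.
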(event `self.ReceiveBeginPlay`
  (`SceneComponent.SetVisibility` (`self.Beam`) false false)
  (`self.Initialize Anim `)
  (if (not (`self.Menu Mode`))
    (`self.Initiate Interact Loop`)))

(event `self.ReceiveTick`
  (params (DeltaSeconds :type "Float (single-precision)"))
  (`self.Movement Tick`))

(event `self.ReceivePossessed`
  (params (NewController :type "Controller Object Reference"))
  (`self.Spawn Inventory Menu`))

(event `Spawn Inventory Menu`
  (if (not (`self.Menu Mode`))
    (bind _asplayer_controller (cast `PlayerController` (`self.GetController`)))
    (bind _returnvalue (`|CreateWidget` "/Game/Widgets/Inventory/UMG_IO_InventoryRibon.UMG_IO_InventoryRibon_C" _asplayer_controller))
    (bind _output_get (set `self.Inv Widget` _returnvalue))
    (`UserWidget.AddToViewport` _output_get 0)
    (`self.Tutorial`)))

(event `Tutorial`
  (`self.Menu Message` "Welcome unit 048" "This new body will facilitate our discovery of what happened to the maker's civilization. ")
  (`KismetSystemLibrary.Delay` 5.0)
  (`self.Menu Message` "Input" "Your rover form is controlled with 10, zzzzttt.... Binary parsing error, 2 buttons, that you will use for input and output. These buttons being the keys 'I' and 'O', or alternativly '1' and '0'.")
  (`KismetSystemLibrary.Delay` 7.0)
  (`self.Menu Message` "Input Continued" "Tapping either button will cycle through your menu. Tapping both buttons will select the highlighted menu option.")
  (`KismetSystemLibrary.Delay` 5.0)
  (`self.Menu Message` "Interaction" "When you come upon an object that can be manipulated a message will be shown here. Tapping both buttons will interact with the object.")
  (`KismetSystemLibrary.Delay` 5.0)
  (`self.Menu Message` "Movement" "To activate the rover's motivator hold the buttons. Holding both will drive forward, holding one will turn in that direction.")
  (`KismetSystemLibrary.Delay` 5.0)
  (`self.Menu Message` "Failure" "Due to lack of resources your rover body has limited power. Make use of local sorounding to scavenge materials and craft what you need to continue. ")
  (`KismetSystemLibrary.Delay` 7.0)
  (`self.Menu Message` "Success" "Once you have found the signal sources do what you need to recover any data contained. When all data is collected return to the drop pod.")
  (`KismetSystemLibrary.Delay` 5.0)
  (`self.Menu Message` "Good luck" "Good Luck")
  (`KismetSystemLibrary.Delay` 2.0)
  (`self.Reset Inventory Menu`))

(event `InputAction|Button 1`
  (params (Key :type "Key Structure"))
  ;[1 1 1] Get raw input and rout it ot buffer if pressed or flag if held
  (:`Pressed`
    (`self.Press or Hold` (`self.Button Hold Delay`) :!label _label
      (:`Hold`
        (set `self.Button 1 Hold` true))
      (:`Pressed`
        (`KismetArrayLibrary.Array_Add` (`self.Button Buffer`) 1)
        (`self.Button Combo Solver` :!label _label_2))))
  (:`Released`
    (set `self.Button 1 Hold` false)
    (goto _label :!via `Release`)))

(event `Button Combo Solver`
  ;[1 1 1] Loop through input buffer and compare to combo strings to trigger desired action. Clear buffer after tests
  (`KismetSystemLibrary.RetriggerableDelay` (`self.Button Exe Delay`))
  (`|ExecutionSequence`
    (:`then_0`
      (`self.Solve Button Combo` (`self.Button 1 Pressed`))
      (`self.Press Button 1`))
    (:`then_1`
      (`self.Solve Button Combo` (`self.Button 2 Pressed`))
      (`self.Press Button 2`))
    (:`then_2`
      (`self.Solve Button Combo` (`self.OpenMenu`))
      (`self.Open Game Menu`))
    (:`then_3`
      (`self.Solve Button Combo` (`self.2 Buttons Pressed`))
      (`self.2 Button Press ` :!label _label_3))
    (:`then_4`
      (`self.Solve Button Combo` (`self.2 Buttons Reversed`))
      (goto _label_3))
    (:`then_5`
      (`KismetArrayLibrary.Array_Clear` (`self.Button Buffer`)))))

(event `CameraSwitch`
  (bind _cameraselect (`self.CameraSelect`))
  (if (== _cameraselect 2)
    (set `self.CameraSelect` 0)
    (else
      (set `self.CameraSelect` (+ _cameraselect 1))))
  (cast `PlayerController` (`self.GetController`))
  (switch `int` (`self.CameraSelect`)
    (:`0`
      (`ActorComponent.SetActive` (`self.Camera0`) true false)
      (`ActorComponent.SetActive` (`self.Camera1`) false false)
      (`ActorComponent.SetActive` (`self.Camera2`) false false))
    (:`1`
      (`ActorComponent.SetActive` (`self.Camera0`) false false)
      (`ActorComponent.SetActive` (`self.Camera1`) true false)
      (`ActorComponent.SetActive` (`self.Camera2`) false false))
    (:`2`
      (`ActorComponent.SetActive` (`self.Camera0`) false false)
      (`ActorComponent.SetActive` (`self.Camera1`) false false)
      (`ActorComponent.SetActive` (`self.Camera2`) true false))))

(event `InputAction|Button 2`
  (params (Key :type "Key Structure"))
  ;[1 1 1] Get raw input and rout it ot buffer if pressed or flag if held
  (:`Pressed`
    (`self.Press or Hold` (`self.Button Hold Delay`) :!label _label_4
      (:`Hold`
        (set `self.Button 2 Hold` true))
      (:`Pressed`
        (`KismetArrayLibrary.Array_Add` (`self.Button Buffer`) 2)
        (goto _label_2))))
  (:`Released`
    (set `self.Button 2 Hold` false)
    (goto _label_4 :!via `Release`)))

(event `Open Game Menu`
  ;[1 1 1] Open main menu
  (set `self.Menu Mode` true)
  (bind _foundwidgets (`WidgetBlueprintLibrary.GetAllWidgetsOfClass` "/Game/Widgets/MainMenu/UMG_IO_GameMenu.UMG_IO_GameMenu_C"))
  (`/Engine/EditorBlueprintResources/StandardMacros.IsValid` null
    (:`Is Valid`
      (set `self.TargetWidget` (`|GetArrayItem` _foundwidgets)))
    (:`Is Not Valid`
      (bind _asplayer_controller (cast `PlayerController` (`self.GetController`)))
      (bind _returnvalue (`|CreateWidget` "/Game/Widgets/MainMenu/UMG_IO_GameMenu.UMG_IO_GameMenu_C" _asplayer_controller))
      (set `self.TargetWidget` _returnvalue)))
  (`UserWidget.AddToViewport` (`self.TargetWidget`) 0))

(event `Press Button 1`
  (if (`self.Menu Mode`)
    (`/Game/Widgets/Class_UMG_IO.Cylcle Prev` (`self.TargetWidget`))
    (elif (not (`self.Building Mode`))
      (`/Engine/EditorBlueprintResources/StandardMacros.IsValid` (`self.Interact Actor`)
        (:`Is Not Valid`
          (`/Game/Widgets/Class_UMG_IO.Cylcle Prev` (`self.Inv Widget`)))))))

(event `Press Button 2`
  (if (`self.Menu Mode`)
    (`/Game/Widgets/Class_UMG_IO.Cycle Next` (`self.TargetWidget`))
    (elif (not (`self.Building Mode`))
      (`/Engine/EditorBlueprintResources/StandardMacros.IsValid` (`self.Interact Actor`)
        (:`Is Not Valid`
          (`/Game/Widgets/Class_UMG_IO.Cycle Next` (`self.Inv Widget`)))))))

(event `2 Button Press`
  (if (`self.Menu Mode`)
    (`/Game/Widgets/Class_UMG_IO.Commit Input Selection` (`self.TargetWidget`))
    (elif (`self.Building Mode`)
      (`self.Craft Build Trigger`)
      (else
        (`/Engine/EditorBlueprintResources/StandardMacros.IsValid` (`self.Interact Actor`)
          (:`Is Valid`
            (`self.Server Request Interact`))
          (:`Is Not Valid`
            (`/Game/Widgets/Class_UMG_IO.Commit Input Selection` (`self.Inv Widget`))))))))

(event `Server Request Interact`
  (bind _interact_actor (`self.Interact Actor`))
  (`/Engine/EditorBlueprintResources/StandardMacros.IsValid` _interact_actor
    (:`Is Valid`
      (message `/Game/Blueprints/Crafting/Interface_Interact.Activate Interact` _interact_actor self)
      (`self.Show Hide Beam` true))))

(event `Movement Tick`
  (if (and (`self.Button 1 Hold`) (`self.Button 2 Hold`))
    (`self.Move Forward`)
    (elif (`self.Button 1 Hold`)
      (`self.Turn Left`)
      (elif (`self.Button 2 Hold`)
        (`self.Turn Right`)))))

(event `Move Forward`
  (`self.AddMovementInput` (`self.GetActorForwardVector`))
  (`self.Drive Treads`)
  (`self.Align Rover`))

(event `Turn Right`
  (`self.AddControllerYawInput` (`self.Turn Rate`))
  (`self.Drive Treads`)
  (`self.Align Rover`))

(event `Turn Left`
  (`self.AddControllerYawInput` (* (`self.Turn Rate`) -1.0))
  (`self.Drive Treads`)
  (`self.Align Rover`))

(event `Initialize Anim`
  (bind _returnvalue (`PrimitiveComponent.CreateDynamicMaterialInstance` (`self.Treads`) 0 "/Game/Materials/Player/MatInst_Treads1.MatInst_Treads1" "None"))
  (set `self.Tread Mat Ref` _returnvalue))

(event `Drive Treads`
  (bind _output_get (set `self.Tread Offset` (+ (`self.Tread Offset`) (`self.Tread Step`))))
  (`MaterialInstanceDynamic.SetScalarParameterValue` (`self.Tread Mat Ref`) "TreadUVOffset" _output_get))

(event `Show Hide Beam`
  (params (`Is Visible` :type Boolean))
  (`SceneComponent.SetVisibility` (`self.Beam`) `Is Visible` false))

(event `Align Rover`
  (bind _returnvalue (`self.K2_GetActorLocation`))
  (bind _rover (`self.Rover`))
  (bind (_outhit _returnvalue_2) (`KismetSystemLibrary.LineTraceSingle` _returnvalue (+ _returnvalue (0.0 0.0 -200.0)) "TraceTypeQuery1"))
  (if _returnvalue_2
    (`SceneComponent.K2_SetWorldRotation` _rover (`KismetMathLibrary.RInterpTo` (`SceneComponent.K2_GetComponentRotation` (`self.Rover`)) (`KismetMathLibrary.MakeRotFromZX` (`.ImpactNormal` (`GameplayStatics.BreakHitResult` _outhit)) (`self.GetActorForwardVector`)) (`GameplayStatics.GetWorldDeltaSeconds`) 5.0) false false)
    (else
      (`SceneComponent.K2_SetWorldRotation` _rover (`self.K2_GetActorRotation`) false false))))

(event `Reset Inventory Menu`
  ;[1 1 1] Return inventory menu to top menu
  (bind _asumg_io_inventory_ribon (cast `/Game/Widgets/Inventory/UMG_IO_InventoryRibon` (`self.Inv Widget`)))
  (`/Game/Widgets/Inventory/UMG_IO_InventoryRibon.Switch Widget` _asumg_io_inventory_ribon 0))

(event `Recieve Resources`
  (params (Resources :type "/Game/Blueprints/Crafting/Harvesting/Struct_HarvestItem Structure"))
  (bind (_displayname _info _wood _metal _wire _parts _chemicals _batteries) (break `/Game/Blueprints/Crafting/Harvesting/Struct_HarvestItem` Resources))
  ;[1 1 1] Add resources to inventory. Stop Harvesting if full
  (`/Engine/EditorBlueprintResources/ActorMacros.Switch Has Authority`
    (:`Authority`
      (`self.Inventoy Full?`
        (:`Full`
          _)
        (:`Has Room`
          (set `self.Wood` (+ _wood (`self.Wood`)))
          (set `self.Metal` (+ _metal (`self.Metal`)))
          (set `self.Wire` (+ _wire (`self.Wire`)))
          (set `self.Parts` (+ _parts (`self.Parts`)))
          (set `self.Chemicals` (+ _chemicals (`self.Chemicals`)))
          (set `self.Batteries` (+ _batteries (`self.Batteries`)))
          (`self.Inventoy Full?`
            (:`Full`
              _))))
      (message `/Game/Blueprints/Crafting/Interface_Interact.EndFocus Interact` (`self.Interact Actor`) self)
      (`self.Menu Message` "Inventory Alert!!!" "Inventory Full")
      (`self.Show Hide Beam` false))))

(event `Initiate Interact Loop`
  ;[1 1 1] Timer loop
  (`KismetSystemLibrary.K2_SetTimerDelegate` (delegate `Trigger Loop`) 0.1 true))

(event `Menu Message`
  (params (Header :type Text) (Info :type Text))
  ;[1 1 1] Display message in inventory window
  (bind _asumg_io_inventory_ribon (cast `/Game/Widgets/Inventory/UMG_IO_InventoryRibon` (`self.Inv Widget`)))
  (`/Game/Widgets/Inventory/UMG_IO_InventoryRibon.Menu Message` _asumg_io_inventory_ribon Header Info))

(event `Trigger Loop`
  ;[1 1 1] Timer loop
  (if (`self.Building Mode`)
    (`self.Building loop`)
    (`self.Craft Local Placement`)
    (else
      (`self.Interact Loop`))))

(event `Interact Loop`
  (bind _trace_emitter (`self.Trace Emitter`))
  (bind _returnvalue (`SceneComponent.K2_GetComponentLocation` _trace_emitter))
  ;[1 1 1] Set target interation actor by line trace. Trigger evensts when actor is set or removed
  (bind (_outhit _returnvalue_2) (`KismetSystemLibrary.LineTraceSingle` _returnvalue (+ _returnvalue (* (`SceneComponent.GetForwardVector` _trace_emitter) (`self.Interact distance`))) "TraceTypeQuery1"))
  (if _returnvalue_2
    (bind (_bblockinghit _binitialoverlap _time _distance _location _impactpoint _normal _impactnormal _physmat _hitactor) (`GameplayStatics.BreakHitResult` _outhit))
    (if (not (== (`self.Interact Actor`) _hitactor))
      (message `/Game/Blueprints/Crafting/Interface_Interact.EndFocus Interact` (`self.Interact Actor`) self)
      (if (`KismetSystemLibrary.DoesImplementInterface` _hitactor "/Game/Blueprints/Crafting/Interface_Interact.Interface_Interact_C")
        (bind _output_get (set `self.Interact Actor` _hitactor))
        (message `/Game/Blueprints/Crafting/Interface_Interact.StartFocus Interact` _output_get self)))
    (else
      (message `/Game/Blueprints/Crafting/Interface_Interact.EndFocus Interact` (`self.Interact Actor`) self)
      (set `self.Interact Actor` null)
      (`/Engine/EditorBlueprintResources/ActorMacros.Switch Has Authority`
        (:`Authority`
          (`self.Show Hide Beam` false))))))

(event `Building loop`
  (bind _returnvalue (+ (`self.K2_GetActorLocation`) (0.0 0.0 100.0)))
  ;[1 1 1] Building Trace
  (bind (_outhit _returnvalue_2) (`KismetSystemLibrary.LineTraceSingle` _returnvalue (+ _returnvalue (* (`self.GetActorForwardVector`) (`self.Build Distance`))) "TraceTypeQuery3" false (`|MakeArray` (`self.CraftActor`))))
  (if _returnvalue_2
    (bind (_bblockinghit _binitialoverlap _time _distance _location _impactpoint _normal _impactnormal _physmat _hitactor _hitcomponent _hitbonename _hititem _faceindex _tracestart _traceend) (`GameplayStatics.BreakHitResult` _outhit))
    (set `self.Build transform` (`KismetMathLibrary.MakeTransform` (+ (* _impactnormal 400.0) (`self.K2_GetActorLocation` _hitactor)) (`KismetMathLibrary.MakeRotFromZX` (`KismetMathLibrary.MakeVector` 0.0 0.0 1.0) (* _impactnormal -1.0))))
    (else
      (set `self.Build transform` (`KismetMathLibrary.MakeTransform` _traceend (`self.K2_GetActorRotation`))))))

(event `Craft Local Placement`
  (`|ExecutionSequence`
    (:`then_0`
      (`/Engine/EditorBlueprintResources/StandardMacros.DoOnce` false :!label _label
        (:`Completed`
          (bind _returnvalue (`|SpawnActorFromClass` (`self.CraftClass`) (`self.Build transform`) "AlwaysSpawn" "OverrideRootScale" null null))
          (set `self.CraftActor` _returnvalue)
          (`KismetSystemLibrary.PrintString` "Create crafting block"))))
    (:`then_1`
      (`self.K2_SetActorTransform` (`self.CraftActor`) (`self.Build transform`) false false))))

(event `Craft Build Trigger`
  (set `self.Building Mode` false)
  (`self.K2_DestroyActor` (`self.CraftActor`))
  (`self.Server Build Item` (`self.CraftClass`) (`self.Build transform`))
  (`self.Reset Inventory Menu`)
  (goto _label :!via `Reset`))

(event `Server Build Item`
  (params (CraftClass :type "Actor Class Reference") (`Build transform` :type "Transform Structure"))
  (bind _returnvalue (`|SpawnActorFromClass` CraftClass `Build transform` "AlwaysSpawn" "OverrideRootScale" self self))
  (bind _asclass_craft_blocks (cast `/Game/Blueprints/Crafting/Building/Class_CraftBlocks` _returnvalue))
  (`/Game/Blueprints/Crafting/Building/Class_CraftBlocks.Fade Out` _asclass_craft_blocks))

(fn `UserConstructionScript`)