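; Example Blueprint that burns away or rebuilds a cube as something enters or leaves its trigger box.
; Overlap begin plays the BurnBuild timeline forward and overlap end reverses it, feeding its track into the "Amount" scalar parameter on the cube's materials.
; A particle system is shown when either direction starts and hidden again when the timeline finishes.
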(event `self.Box.OnComponentBeginOverlap`
  (params (OverlappedComponent :type "PrimitiveComponent Object Reference") (OtherActor :type "Actor Object Reference") (OtherComp :type "PrimitiveComponent Object Reference") (OtherBodyIndex :type Integer) (bFromSweep :type Boolean) (SweepResult :type "HitResult Structure (by ref)"))
  (`self.Burn`))

(event `Burn`
  (`SceneComponent.SetHiddenInGame` (`self.ParticleSystem`) false false)
  (bind (_direction _newtrack_0) (`Timeline|Burn/Build` :!label _label)
    (:`Update`
      (`MeshComponent.SetScalarParameterValueOnMaterials` (`self.Cube`) "Amount" _newtrack_0))
    (:`Finished`
      (`SceneComponent.SetHiddenInGame` (`self.ParticleSystem`) true false))))

(event `Build`
  (`SceneComponent.SetHiddenInGame` (`self.ParticleSystem`) false false)
  (goto _label :!via `Reverse`))

(event `self.Box.OnComponentEndOverlap`
  (params (OverlappedComponent :type "PrimitiveComponent Object Reference") (OtherActor :type "Actor Object Reference") (OtherComp :type "PrimitiveComponent Object Reference") (OtherBodyIndex :type Integer))
  (`self.Build`))

(fn `UserConstructionScript`)