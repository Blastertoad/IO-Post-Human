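; Player character Blueprint for a treaded drone with tank-style controls on A and D.
; Key flags and the InputLeft and InputRight axis events move it forward when both keys are held, otherwise yaw it by axis value.
; While either key is held, the axis events scroll the treads through a UV offset parameter on a dynamic material created at BeginPlay.
; One material drives the treads, so they cannot animate independently.
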(event `self.ReceiveBeginPlay`
  ;[1 1 1] Tread Material
  (bind _returnvalue (`PrimitiveComponent.CreateDynamicMaterialInstance` (`self.DroneTreads`) 0 "/Game/Character/DroneModel/Treads1_Inst.Treads1_Inst" "None"))
  (set `self.TreadMatRef` _returnvalue))

(event `Key|A` :consume false
  (params (Key :type "Key Structure"))
  ;[1 1 1] Consume Input Off
  (:`Pressed`
    ;[1 1 1] Check to see if both keys are held down
    (set `self.A Held` true))
  (:`Released`
    (set `self.A Held` false)))

(event `InputAxis|InputLeft` :consume false
  (params (AxisValue :type "Float (single-precision)"))
  ;[1 1 1] Consume Input Off
  ;[1 1 1] Check to see if both keys are held down
  (if (and (`self.A Held`) (`self.D Held`))
    ;[1 1 1] Forward if both keys held down
    (`self.K2_AddActorLocalOffset` (`KismetMathLibrary.MakeVector` (`self.Forward Speed`)) :!label _label)
    (else
      ;[1 1 1] Turn Left
      (`self.K2_AddActorLocalRotation` (`KismetMathLibrary.MakeRotator` 0.0 0.0 (* (`self.Rotation Speed`) (* AxisValue -1.0))))))
  ;[1 1 1] Controls treads. To get indepedant tread movement I need 2 materials on the treads and then would control each individually based on input.
  (if (or (`self.A Held`) (`self.D Held`)) :!label _label_2
    (bind _output_get (set `self.TreadsPositionOffset` (+ (`self.TreadsPositionOffset`) (`self.TreadSpeed`))))
    (`MaterialInstanceDynamic.SetScalarParameterValue` (`self.TreadMatRef`) "TreadUVOffset" _output_get)))

(event `InputAxis|InputRight` :consume false
  (params (AxisValue :type "Float (single-precision)"))
  ;[1 1 1] Consume Input Off
  ;[1 1 1] Check to see if both keys are held down
  (if (and (`self.A Held`) (`self.D Held`))
    (goto _label)
    (else
      ;[1 1 1] Turn Right
      (`self.K2_AddActorLocalRotation` (`KismetMathLibrary.MakeRotator` 0.0 0.0 (* AxisValue (`self.Rotation Speed`))))
      (goto _label_2))))

(event `Key|D` :consume false
  (params (Key :type "Key Structure"))
  ;[1 1 1] Consume Input Off
  (:`Pressed`
    ;[1 1 1] Check to see if both keys are held down
    (set `self.D Held` true))
  (:`Released`
    (set `self.D Held` false)))

(fn `UserConstructionScript`)